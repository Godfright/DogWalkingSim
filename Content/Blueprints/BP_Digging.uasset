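; BP_Digging is a dig spot actor that tries to spawn a random item when BP_CorgiBT overlaps its Collision component.
; ItemSpawning spawns BP_Items there with a DT_Items mesh, but picks from column names instead of row names and is noted as not working.
; An ItemSpawn function uses row names but is not called here.
; Disconnected logic would toggle the AI's CanDig blackboard key.
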(event OnComponentBeginOverlap(Collision)
  (params (OverlappedComponent :type Primitive%20Component%20Object%20Reference) (OtherActor :type Actor%20Object%20Reference) (OtherComp :type Primitive%20Component%20Object%20Reference) (OtherBodyIndex :type Integer) (bFromSweep :type Boolean) (SweepResult :type Hit%20Result%20Structure%20%28by%20ref%29))
  ;[1 1 1 0.502] Item Spawn Didn't work
  (Utilities|Casting|CastToBP_CorgiBT OtherActor)
  (CallFunction|ItemSpawning))

(event Custom|ItemSpawning
  ;[1 1 1 0.502] Item Spawn Didn't work
  (bind _outcolumnnames (Class|DataTableFunctionLibrary|GetDataTableColumnNames "/Game/DataTables/DT_Items.DT_Items"))
  (bind _returnvalue (Utilities|GetDataTableRow "/Game/DataTables/DT_Items.DT_Items" (.OutItem (Utilities|Array|Random _outcolumnnames)))
    (:then
      (bind _returnvalue_2 (Game|SpawnActorfromClass "/Game/DataTables/BP_Items.BP_Items_C" (Math|Transform|MakeTransform (Transformation|GetWorldLocation (Variables|Default|GetCollision)) "0, 0, 0" "1.000000,1.000000,1.000000") "Undefined" "MultiplyWithRoot" 0 0))
      (Components|StaticMesh|SetStaticMesh (Variables|/Game/DataTables/BP_Items.BP_Items_C|GetItem _returnvalue_2) (.itemmesh _returnvalue)))))

(event EventBeginPlay)

(event Collision|EventActorBeginOverlap
  (params (OtherActor :type Actor%20Object%20Reference)))

(event Collision|EventActorEndOverlap
  (params (OtherActor :type Actor%20Object%20Reference)))

(fn ConstructionScript)

(fn ItemSpawn
  (params (StaticMesh :type Static%20Mesh%20Object%20Reference))
  (bind _outrownames (DataTable|GetDataTableRowNames "/Game/DataTables/DT_Items.DT_Items"))
  (Utilities|GetDataTableRow "/Game/DataTables/DT_Items.DT_Items" (.OutItem (Utilities|Array|Random _outrownames))
    (:then
      (bind _returnvalue (Game|SpawnActorfromClass "/Game/DataTables/BP_Items.BP_Items_C" (Math|Transform|MakeTransform "0, 0, 0" "0, 0, 0" "1.000000,1.000000,1.000000") "Undefined" "MultiplyWithRoot" 0 0))
      (Components|StaticMesh|SetStaticMesh (Variables|/Game/DataTables/BP_Items.BP_Items_C|GetItem _returnvalue) StaticMesh))))