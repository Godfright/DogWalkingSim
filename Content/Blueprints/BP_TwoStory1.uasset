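; BP_TwoStory1 is a building Blueprint with a door that shows a press-E prompt and is meant to load another level.
; It creates the W_PressEDoor widget at BeginPlay, then adds or removes it as the player enters or leaves DoorCollision.
; The E key handler, commented "Failed", opens TestingScale with debug prints if IsPlayerNear is true, but nothing here sets that flag.
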(event OnComponentBeginOverlap(DoorCollision)
  (params (OverlappedComponent :type Primitive%20Component%20Object%20Reference) (OtherActor :type Actor%20Object%20Reference) (OtherComp :type Primitive%20Component%20Object%20Reference) (OtherBodyIndex :type Integer) (bFromSweep :type Boolean) (SweepResult :type Hit%20Result%20Structure%20%28by%20ref%29))
  (if (== OtherActor (Game|GetPlayerCharacter 0))
    (UserInterface|Viewport|AddtoViewport (Variables|Default|GetPressE) 0)))

(event OnComponentEndOverlap(DoorCollision)
  (params (OverlappedComponent :type Primitive%20Component%20Object%20Reference) (OtherActor :type Actor%20Object%20Reference) (OtherComp :type Primitive%20Component%20Object%20Reference) (OtherBodyIndex :type Integer))
  (if (== (Game|GetPlayerCharacter 0) OtherActor)
    (Widget|RemovefromParent (Variables|Default|GetPressE))))

(event EventBeginPlay
  (bind _returnvalue (UserInterface|CreateWidget "/Game/Widgets/W_PressEDoor.W_PressEDoor_C"))
  (Variables|Default|SetPressE _returnvalue))

(event Input|KeyboardEvents|E
  (params (Key :type Key%20Structure :default "None"))
  ;[1 1 1 0.502] Failed
  (:Pressed
    (if (Variables|Default|GetIsPlayerNear?)
      (Development|PrintString "LevelSUCCESS")
      (Game|OpenLevel(byName) "TestingScale")
      (Development|PrintString "LevelFAIL" true true "(R=0.375000,G=0.008137,B=0.000000,A=1.000000)"))))

(fn ConstructionScript)