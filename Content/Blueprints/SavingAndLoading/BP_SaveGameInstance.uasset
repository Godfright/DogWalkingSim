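; Game instance that owns the current BP_SaveGame object and handles creating, saving and loading it in a named slot.
; RequestSave passes all BPI_Savable actors to the save object before writing, and RequestLoad has it restore data for one requester.
; Saving and loading run sync or async and fire GameSaved or GameLoaded.
; Async load continues from the immediate Then pin, not Completed as async save does.
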(event Custom|SaveGame
  (params (Async :type Boolean))
  (bind _savegameref (Variables|Default|GetSaveGameRef))
  ;[1 1 1 0.5] Save the file to hard drive with latest information
  (if Async
    (|AsyncSaveGametoSlot (Variables|Default|GetSaveGameRef) (Variables|Default|GetSaveGameSlotName)
      (:Completed
        (Default|CallGameSaved _savegameref)))
    (else
      (SaveGame|SaveGametoSlot (Variables|Default|GetSaveGameRef) (Variables|Default|GetSaveGameSlotName))
      (Default|CallGameSaved _savegameref))))

(event Custom|CreateSaveGame
  ;[1 1 1 0.5] When 'NEW' is clicked, it will create a SaveGameObject
  (bind _returnvalue (SaveGame|CreateSaveGameObject "/Game/Blueprints/SavingAndLoading/BP_SaveGame.BP_SaveGame_C"))
  (Variables|Default|SetSaveGameRef _returnvalue))

(event Custom|LoadGame
  (params (Async :type Boolean))
  ;[1 1 1 0.502] Ability to load in a file
  (bind _returnvalue (SaveGame|DoesSaveGameExist (Variables|Default|GetSaveGameSlotName)))
  (if _returnvalue
    (if Async
      (bind _savegame (|AsyncLoadGamefromSlot (Variables|Default|GetSaveGameSlotName))
        (:then
          (bind _asbp_save_game (Utilities|Casting|CastToBP_SaveGame _savegame))
          (bind _output_get (Variables|Default|SetSaveGameRef _asbp_save_game))
          (Default|CallGameLoaded _output_get)))
      (else
        (bind _returnvalue_2 (SaveGame|LoadGamefromSlot (Variables|Default|GetSaveGameSlotName)))
        (bind _asbp_save_game_2 (Utilities|Casting|CastToBP_SaveGame _returnvalue_2))
        (bind _output_get_2 (Variables|Default|SetSaveGameRef _asbp_save_game_2))
        (Default|CallGameLoaded _output_get_2)))))

(event EventRequestSave
  (params (Async :type Boolean))
  ;[1 1 1 0.502] Updated SaveGame object with latest information
  (bind _outactors (Actor|GetAllActorswithInterface "/Game/Blueprints/SavingAndLoading/BPI_Savable.BPI_Savable_C"))
  (Default|SaveAllData (Variables|Default|GetSaveGameRef) _outactors)
  (CallFunction|SaveGame Async))

(event EventRequestLoad
  (params (Requester :type Object%20Object%20Reference))
  (Default|LoadDataforRequester (Variables|Default|GetSaveGameRef) Requester))