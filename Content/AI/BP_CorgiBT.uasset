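; Corgi AI pawn that can follow the player and dig up random items, with Pawn Sensing feeding its Blackboard.
; Seeing the third-person player sets a "HasSeenPlayer?" flag, while FollowPlayer re-issues AIMoveTo after each successful move.
; DigItemNew spawns a BP_Items actor with a mesh from a random DT_Items row.
; The DigItem function is an empty stub, referenced only by disconnected nodes.
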(event OnSeePawn(PawnSensing)
  (params (Pawn :type Pawn%20Object%20Reference))
  (Utilities|Casting|CastToBP_ThirdPersonCharacter Pawn)
  (AI|Components|Blackboard|SetValueasBool (AI|GetBlackboard (AI|GetAIController self)) (Utilities|Name|MakeLiteralName "HasSeenPlayer?") true))

(event Custom|FollowPlayer
  ;[0.15 0.15 0.15 0.5] Allows AI (Corgi) to follow the player
  (AI|AIMoveTo self "0, 0, 0" (Game|GetPlayerCharacter 0) 5.0 false
    (:OnSuccess
      (CallFunction|FollowPlayer))))

(event Custom|DigItemNew
  (bind _outrownames (DataTable|GetDataTableRowNames "/Game/DataTables/DT_Items.DT_Items"))
  (bind _returnvalue (Utilities|GetDataTableRow "/Game/DataTables/DT_Items.DT_Items" (.OutItem (Utilities|Array|Random _outrownames)))
    (:then
      (bind _returnvalue_2 (Game|SpawnActorfromClass "/Game/DataTables/BP_Items.BP_Items_C" (Math|Transform|MakeTransform "0, 0, 0" "0, 0, 0" "1.000000,1.000000,1.000000") "Undefined" "MultiplyWithRoot" 0 0))
      (Components|StaticMesh|SetStaticMesh (Variables|/Game/DataTables/BP_Items.BP_Items_C|GetItem _returnvalue_2) (.itemmesh _returnvalue)))))

(fn ConstructionScript)

(fn DigItem)