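; BP_Corgi is an AI corgi pawn that detects the player character through pawn sensing.
; On seeing a BP_ThirdPersonCharacter, it sets the "HasSeenPlayer?" Blackboard key on its AI controller to true.
; A FollowPlayer event moves it to the player and repeats on each success, but its only outside call is disconnected.
; The name tag overlap events, BeginPlay and construction script are empty.
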(event OnSeePawn(PawnSensing)
  (params (Pawn :type Pawn%20Object%20Reference))
  (Utilities|Casting|CastToBP_ThirdPersonCharacter Pawn)
  (AI|Components|Blackboard|SetValueasBool (AI|GetBlackboard (AI|GetAIController self)) (Utilities|Name|MakeLiteralName "HasSeenPlayer?") true))

(event OnComponentBeginOverlap(NameTagCollision)
  (params (OverlappedComponent :type Primitive%20Component%20Object%20Reference) (OtherActor :type Actor%20Object%20Reference) (OtherComp :type Primitive%20Component%20Object%20Reference) (OtherBodyIndex :type Integer) (bFromSweep :type Boolean) (SweepResult :type Hit%20Result%20Structure%20%28by%20ref%29)))

(event OnComponentEndOverlap(NameTagCollision)
  (params (OverlappedComponent :type Primitive%20Component%20Object%20Reference) (OtherActor :type Actor%20Object%20Reference) (OtherComp :type Primitive%20Component%20Object%20Reference) (OtherBodyIndex :type Integer)))

(event Custom|FollowPlayer
  ;[0.15 0.15 0.15 0.5] Allows AI (Corgi) to follow the player
  (AI|AIMoveTo self "0, 0, 0" (Game|GetPlayerCharacter 0) 5.0 false
    (:OnSuccess
      (CallFunction|FollowPlayer))))

(event EventBeginPlay)

(fn ConstructionScript)